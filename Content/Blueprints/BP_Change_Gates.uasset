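; BP_Change_Gates is a gate actor that swaps the red and green light materials between its Green and Red components on each Box begin overlap.
; The ColorSwap variable toggles between two states to choose which component gets which material, with no filter on the overlapping actor.
; BeginPlay creates and stores dynamic material instances for both components, but the swap applies the base materials directly and never uses those instances.
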(event `self.ReceiveBeginPlay`
  (bind _returnvalue (`PrimitiveComponent.CreateDynamicMaterialInstance` (`self.green`) 0 "/Game/Material/M_GreenLight.M_GreenLight" "None"))
  (set `self.NewVar_1` _returnvalue)
  (bind _returnvalue_2 (`PrimitiveComponent.CreateDynamicMaterialInstance` (`self.red`) 0 "/Game/Material/M_RedLight.M_RedLight" "None"))
  (set `self.NewVar_0` _returnvalue_2))

(event `self.Box.OnComponentBeginOverlap`
  (params (OverlappedComponent :type "PrimitiveComponent Object Reference") (OtherActor :type "Actor Object Reference") (OtherComp :type "PrimitiveComponent Object Reference") (OtherBodyIndex :type Integer) (bFromSweep :type Boolean) (SweepResult :type "HitResult Structure (by ref)"))
  (if (== (`self.Color_Swap`) 1)
    (`PrimitiveComponent.SetMaterial` (`self.green`) 0 "/Game/Material/M_RedLight.M_RedLight")
    (`PrimitiveComponent.SetMaterial` (`self.red`) 0 "/Game/Material/M_GreenLight.M_GreenLight")
    (set `self.Color_Swap` 2)
    (else
      (`PrimitiveComponent.SetMaterial` (`self.red`) 0 "/Game/Material/M_RedLight.M_RedLight")
      (`PrimitiveComponent.SetMaterial` (`self.green`) 0 "/Game/Material/M_GreenLight.M_GreenLight")
      (set `self.Color_Swap` 1))))

(fn `UserConstructionScript`)