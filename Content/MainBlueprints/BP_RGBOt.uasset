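; BP_RGBOt is a movable pawn whose cube mesh switches between green and red light materials.
; Forward/back and right/left input axes feed movement input along the actor's own forward and right vectors.
; Tick polls the Color variable and reapplies the matching material to Cube2 every frame; nothing here changes Color.
; BeginPlay also creates and stores a dynamic red-light material instance, which no other logic uses.
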(event `self.ReceiveBeginPlay`
  (bind _returnvalue (`PrimitiveComponent.CreateDynamicMaterialInstance` (`self.Cube2`) 0 "/Game/Material/M_RedLight.M_RedLight" "None"))
  (set `self.NewVar_0` _returnvalue))

(event `self.ReceiveTick`
  (params (DeltaSeconds :type "Float (single-precision)"))
  (bind _color (`self.Color`))
  (bind _cube2 (`self.Cube2`))
  (if (== _color 1)
    (`PrimitiveComponent.SetMaterial` _cube2 0 "/Game/Material/M_GreenLight.M_GreenLight")
    (elif (== _color 2)
      (`PrimitiveComponent.SetMaterial` _cube2 0 "/Game/Material/M_RedLight.M_RedLight"))))

(event `InputAxis|Forward&Backward`
  (params (AxisValue :type "Float (single-precision)"))
  (`self.AddMovementInput` (`self.GetActorForwardVector`) AxisValue))

(event `InputAxis|Right&Left`
  (params (AxisValue :type "Float (single-precision)"))
  (`self.AddMovementInput` (`self.GetActorRightVector`) AxisValue))

(fn `UserConstructionScript`)